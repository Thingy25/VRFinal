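; BP_Duck1 is a shootable duck target that awards tutorial score.
; Tick repeatedly runs a short Delay and plays the TL_DuckFloat timeline, which moves BaseMesh along relative Y, scaled by SpeedMultiplier.
; When a FirstPersonProjectile hits the Capsule, it increments TutorialScore on the BP_PLayer3 player, prints the score, plays a shattered-glass sound and destroys itself.
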(event `self.ReceiveTick`
  (params (DeltaSeconds :type "Float (single-precision)"))
  (`KismetSystemLibrary.Delay` 0.5)
  (bind (_direction _floatval) (`Timeline|TL_DuckFloat`)
    (:`Update`
      (`SceneComponent.K2_SetRelativeLocation` (`self.BaseMesh`) (`KismetMathLibrary.MakeVector` 0.0 (* _floatval (`self.speedMultiplier`))) false false))))

(event `self.Capsule.OnComponentHit`
  (params (HitComponent :type "PrimitiveComponent Object Reference") (OtherActor :type "Actor Object Reference") (OtherComp :type "PrimitiveComponent Object Reference") (NormalImpulse :type "Vector Structure") (Hit :type "HitResult Structure (by ref)"))
  (cast `/Game/FirstPersonBP/Blueprints/FirstPersonProjectile` OtherActor)
  (bind _asbp_player_3 (cast `/Game/FirstPersonBP/Blueprints/BP_PLayer3` (`GameplayStatics.GetPlayerCharacter` 0)))
  (bind _output_get (set `/Game/FirstPersonBP/Blueprints/BP_PLayer3.tutorialScore` (+ (`/Game/FirstPersonBP/Blueprints/BP_PLayer3.tutorialScore` _asbp_player_3) 1.0) _asbp_player_3))
  (`KismetSystemLibrary.PrintString` (`KismetStringLibrary.Conv_DoubleToString` _output_get))
  (`GameplayStatics.PlaySoundAtLocation` "/Game/Audio/ShatteredGlass.ShatteredGlass" (`SceneComponent.K2_GetComponentLocation` (`self.BaseMesh`)) (struct) 1.0 1.0 0.0 null null null)
  (`self.K2_DestroyActor`))

(fn `UserConstructionScript`)