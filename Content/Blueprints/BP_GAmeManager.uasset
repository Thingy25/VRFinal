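; BP_GAmeManager is a game manager Blueprint that runs a minutes-and-seconds countdown.
; Tick feeds a one-second Delay, which ignores calls while pending, so the countdown steps roughly once per second.
; Each step decrements Secs, or borrows a minute from Mins when Secs reaches zero.
; The count stops changing when both reach zero, with no event fired; BeginPlay and the construction script are empty.
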(event `self.ReceiveTick`
  (params (DeltaSeconds :type "Float (single-precision)"))
  (`KismetSystemLibrary.Delay` 1.0)
  (if (== (`self.secs`) 0)
    (if (not (== (`self.mins`) 0))
      (set `self.secs` 59)
      (set `self.mins` (- (`self.mins`) 1)))
    (else
      (set `self.secs` (- (`self.secs`) 1)))))

(fn `UserConstructionScript`)